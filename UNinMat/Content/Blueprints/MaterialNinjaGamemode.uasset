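; Game mode for Material Ninja that handles level setup and world reset on player respawn.
; BeginPlay calls Cloaking on every Tile_Blocking actor.
; RespawnPlayer re-enables and clears the DisabledActor list, then teleports each MaterialBox mesh to its original transform and applies damage to the box.
; LevelLoad is unfinished: it looks up a LevelTable row by index but does nothing with it.
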(event Custom|RespawnPlayer
  (Utilities|FlowControl|Sequence
    (:then_0
      (for _array_element (Variables|Default|GetDisabledActor)
        (CallFunction|EnableActor _array_element))
      (Utilities|Array|Clear (Variables|Default|GetDisabledActor)))
    (:then_1
      (bind _outactors (Actor|GetAllActorsOfClass "/Game/Blueprints/MaterialBox.MaterialBox_C"))
      (for _array_element_2 _outactors
        (Transformation|SetWorldTransform (Variables|/Game/Blueprints/MaterialBox.MaterialBox_C|GetMesh _array_element_2) (Variables|/Game/Blueprints/MaterialBox.MaterialBox_C|GetOriPos _array_element_2) false true)
        (Game|Damage|ApplyDamage _array_element_2 1.0 0 0)))))

(event Custom|LevelLoad
  (params (LevelIndex :type Integer))
  (bind _returnvalue (Utilities|GetDataTableRow "/Game/Blueprints/LevelTable.LevelTable" (Utilities|String|StringToName (Utilities|String|ToString(Integer) LevelIndex)))))

(event EventBeginPlay
  (bind _outactors (Actor|GetAllActorsOfClass "/Game/Blueprints/Tiles/Tile_Blocking.Tile_Blocking_C"))
  (for _array_element _outactors
    (Default|Cloaking _array_element)))

(event EventTick
  (params (DeltaSeconds :type Float%20%28single-precision%29)))

(fn ConstructionScript)