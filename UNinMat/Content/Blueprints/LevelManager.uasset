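; LevelManager saves and loads a level layout to a file in the project directory.
; SaveLevel scans all actors and writes each one whose class is in the game instance's ClassTable as four strings: table index and X, Y, Z location.
; loadlev reads the list in groups of four and spawns those classes at the saved locations with default rotation and scale, without clearing existing actors.
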(event Custom|SaveLevel
  (bind _leveldata (Variables|Default|GetLevelData))
  (Utilities|Array|Clear (Variables|Default|GetLevelData))
  (bind _outactors (Actor|GetAllActorsOfClass "/Script/Engine.Actor"))
  (for _array_element _outactors
    (if (> (Utilities|Array|FindItem (Variables|/Game/Blueprints/ClassTable.ClassTable_C|GetActorClassTable (Variables|Default|GetCT)) (Utilities|GetClass _array_element)) -1)
      (Utilities|Array|Add _leveldata (Utilities|String|ToString(Integer) (Utilities|Array|FindItem (Variables|/Game/Blueprints/ClassTable.ClassTable_C|GetActorClassTable (Variables|Default|GetCT)) (Utilities|GetClass _array_element))))
      (Utilities|Array|Add _leveldata (Utilities|String|ToString(Float) (.x (Transformation|GetActorLocation _array_element))))
      (Utilities|Array|Add _leveldata (Utilities|String|ToString(Float) (.y (Transformation|GetActorLocation _array_element))))
      (Utilities|Array|Add _leveldata (Utilities|String|ToString(Float) (.z (Transformation|GetActorLocation _array_element))))))
  (bind _returnvalue (Class|LevelCreater|WriteLeveltoFile (Variables|Default|GetLevelData) (Class|BlueprintPathsLibrary|ProjectDir) (Variables|Default|GetfileName)))
  (bind _output_get (Variables|Default|SetFileResult _returnvalue))
  (if _output_get
    (Development|PrintString "SaveComplete")))

(event Custom|loadlev
  (Utilities|Array|Clear (Variables|Default|GetLevelData))
  (bind (_target _returnvalue) (Class|LevelCreater|ReadLevelfromFile (Class|BlueprintPathsLibrary|ProjectDir) (Variables|Default|GetfileName)))
  (bind _output_get (Variables|Default|SetFileResult _returnvalue))
  (if _output_get
    (for (_array_element _array_index) _target
      (switch int (Math|Integer|%(Integer) _array_index 4)
        (:0
          (bind _output_get_2 (Variables|Default|SetClassIndex (Math|Float|Truncate (Math|Conversions|ToFloat(Integer) _array_element)))))
        (:1
          (bind _output_get_3 (Variables|Default|SetfloatX (Math|Conversions|ToFloat(Integer) _array_element))))
        (:2
          (bind _output_get_4 (Variables|Default|SetfloatY (Math|Conversions|ToFloat(Integer) _array_element))))
        (:3
          (bind _output_get_5 (Variables|Default|SetfloatZ (Math|Conversions|ToFloat(Integer) _array_element)))
          (Game|SpawnActorfromClass (Utilities|Array|Get(acopy) (Variables|/Game/Blueprints/ClassTable.ClassTable_C|GetActorClassTable (Variables|Default|GetCT)) _output_get_2) (Math|Transform|MakeTransform (Math|Vector|MakeVector _output_get_3 _output_get_4 _output_get_5)) "Undefined" 0 0))))
    (Development|PrintString "LoadComplete")
    (else
      (Development|PrintString "LoadFailed"))))

(event EventBeginPlay
  (bind _asclass_table (Utilities|Casting|CastToClassTable (Game|GetGameInstance)))
  (Variables|Default|SetCT _asclass_table))

(event Collision|EventActorBeginOverlap
  (params (OtherActor :type Actor%20Object%20Reference)))

(event EventTick
  (params (DeltaSeconds :type Float%20%28single-precision%29)))

(fn ConstructionScript)