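; Shuriken projectile actor that transfers its material to any MaterialBox it hits.
; Tick spins the mesh and slides the root along world Y in its facing direction by MovementSpeed, without sweep or delta-time scaling.
; When Shooted is set, a Box overlap with a MaterialBox copies MyMatInfo and its material onto that box, then destroys the shuriken.
; Other overlaps are ignored, as the PlayerCharacter check is unwired.
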(event OnComponentBeginOverlap(Box)
  (params (OverlappedComponent :type Primitive%20Component%20Object%20Reference) (OtherActor :type Actor%20Object%20Reference) (OtherComp :type Primitive%20Component%20Object%20Reference) (OtherBodyIndex :type Integer) (bFromSweep :type Boolean) (SweepResult :type Hit%20Result%20Structure%20%28by%20ref%29))
  (if (Variables|Default|GetShooted)
    (bind _asmaterial_box (Utilities|Casting|CastToMaterialBox OtherActor))
    (Variables|/Game/Blueprints/MaterialBox.MaterialBox_C|SetMyMatInfo _asmaterial_box (Variables|Default|GetMyMatInfo))
    (Rendering|Material|SetMaterial (Variables|/Game/Blueprints/MaterialBox.MaterialBox_C|GetMesh _asmaterial_box) 0 (.material (Variables|Default|GetMyMatInfo)))
    (Actor|DestroyActor)))

(event EventBeginPlay)

(event Collision|EventActorBeginOverlap
  (params (OtherActor :type Actor%20Object%20Reference)))

(event EventTick
  (params (DeltaSeconds :type Float%20%28single-precision%29))
  (bind _sceneroot (Variables|Default|GetSceneRoot))
  (Transformation|AddRelativeRotation (Variables|Default|GetMesh) "0,10.000000, 0" false false)
  (Utilities|IsValid _sceneroot
    (:Is%20Valid
      (Transformation|AddWorldOffset _sceneroot (* (Math|Vector|Normalize (Math|Vector|MakeVector 0.0 (.y (Math|Vector|GetForwardVector _sceneroot)) 0.0)) (Variables|Default|GetMovementSpeed)) false false))))

(fn ConstructionScript)