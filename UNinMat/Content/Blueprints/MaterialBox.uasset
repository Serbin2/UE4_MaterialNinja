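; MaterialBox is a box that player characters can push sideways if their Weight meets or exceeds its material's Weight.
; Overlaps on LeftCol and RightCol set push flags; Tick then shifts the mesh by the player's MovementSize, doubling Y, when direction matches.
; BeginPlay stores the mesh's transform and disables physics under LevelEditorGamemode.
; Any damage teleports the actor to that transform and applies the Wood data-table row's info and material.
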(event OnComponentBeginOverlap(LeftCol)
  (params (OverlappedComponent :type Primitive%20Component%20Object%20Reference) (OtherActor :type Actor%20Object%20Reference) (OtherComp :type Primitive%20Component%20Object%20Reference) (OtherBodyIndex :type Integer) (bFromSweep :type Boolean) (SweepResult :type Hit%20Result%20Structure%20%28by%20ref%29))
  (bind _asplayer_character (Utilities|Casting|CastToPlayerCharacter OtherActor))
  (if (>= (.weight (Variables|/Game/Blueprints/PlayerCharacter.PlayerCharacter_C|GetMyInfo _asplayer_character)) (.weight (Variables|Default|GetMyMatInfo)))
    (Variables|Default|SetRightPush true)
    (Variables|Default|SetPC _asplayer_character)))

(event OnComponentEndOverlap(LeftCol)
  (params (OverlappedComponent :type Primitive%20Component%20Object%20Reference) (OtherActor :type Actor%20Object%20Reference) (OtherComp :type Primitive%20Component%20Object%20Reference) (OtherBodyIndex :type Integer))
  (Utilities|Casting|CastToPlayerCharacter OtherActor)
  (Variables|Default|SetRightPush false))

(event OnComponentBeginOverlap(RightCol)
  (params (OverlappedComponent :type Primitive%20Component%20Object%20Reference) (OtherActor :type Actor%20Object%20Reference) (OtherComp :type Primitive%20Component%20Object%20Reference) (OtherBodyIndex :type Integer) (bFromSweep :type Boolean) (SweepResult :type Hit%20Result%20Structure%20%28by%20ref%29))
  (bind _asplayer_character (Utilities|Casting|CastToPlayerCharacter OtherActor))
  (if (>= (.weight (Variables|/Game/Blueprints/PlayerCharacter.PlayerCharacter_C|GetMyInfo _asplayer_character)) (.weight (Variables|Default|GetMyMatInfo)))
    (Variables|Default|SetLeftPush true)
    (Variables|Default|SetPC _asplayer_character)))

(event OnComponentEndOverlap(RightCol)
  (params (OverlappedComponent :type Primitive%20Component%20Object%20Reference) (OtherActor :type Actor%20Object%20Reference) (OtherComp :type Primitive%20Component%20Object%20Reference) (OtherBodyIndex :type Integer))
  (Utilities|Casting|CastToPlayerCharacter OtherActor)
  (Variables|Default|SetLeftPush false))

(event EventBeginPlay
  (Utilities|FlowControl|Sequence
    (:then_0
      (Utilities|Casting|CastToLevelEditorGamemode (Game|GetGameMode))
      (Physics|SetSimulatePhysics (Variables|Default|GetMesh) false))
    (:then_1
      (Variables|Default|SetOriPos (Transformation|GetWorldTransform (Variables|Default|GetMesh))))))

(event Collision|EventActorBeginOverlap
  (params (OtherActor :type Actor%20Object%20Reference)))

(event EventTick
  (params (DeltaSeconds :type Float%20%28single-precision%29))
  (bind _pc (Variables|Default|GetPC))
  (bind _movementsize (Variables|/Game/Blueprints/PlayerCharacter.PlayerCharacter_C|GetMovementSize _pc))
  (Utilities|FlowControl|Sequence
    (:then_0
      (if (Variables|Default|GetRightPush)
        (if (< (.y _movementsize) 0.0)
          (Transformation|SetWorldLocation (Variables|Default|GetMesh) (+ (Transformation|GetWorldLocation (Variables|Default|GetMesh)) (Math|Vector|MakeVector (.x _movementsize) (* (.y _movementsize) 2.0) (.z _movementsize))) false false :!label _label))))
    (:then_1
      (if (Variables|Default|GetLeftPush)
        (if (> (.y _movementsize) 0.0)
          (goto _label))))))

(event Game|Damage|EventAnyDamage
  (params (Damage :type Float%20%28single-precision%29) (DamageType :type Damage%20Type%20Object%20Reference) (InstigatedBy :type Controller%20Object%20Reference) (DamageCauser :type Actor%20Object%20Reference))
  (Transformation|SetActorTransform (Variables|Default|GetOriPos) false true)
  (bind _returnvalue (Utilities|GetDataTableRow "/Game/Blueprints/MaterialInfoTable.MaterialInfoTable" "Wood")
    (:then
      (bind _output_get (Variables|Default|SetMyMatInfo _returnvalue))
      (Rendering|Material|SetMaterial (Variables|Default|GetMesh) 0 (.Material (Utilities|Struct|BreakMaterialInfo _output_get))))))

(fn ConstructionScript)