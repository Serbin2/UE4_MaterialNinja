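; Player character for an in-game level editor that moves along a grid of blank tiles and places or deletes actors on them.
; BeginPlay spawns the Y-Z tile grid, creates the editor HUD and finds the LevelManager.
; HUD events and hotkeys create or destroy the actor on SelectedTile, which records what it holds.
; Ctrl shortcuts drive LevelManager to save, load or advance levels, exchanging name and creator text with the HUD.
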(event Custom|DeleteTile
  (bind _selectedtile (Variables|Default|GetSelectedTile))
  (if (Variables|Default|GetHoldingTile)
    (if (Variables|/Game/Blueprints/Tiles/Tile_Blank.Tile_Blank_C|GetisTilePlaced _selectedtile)
      (Actor|DestroyActor (Variables|/Game/Blueprints/Tiles/Tile_Blank.Tile_Blank_C|GetPlacedTile _selectedtile))
      (Variables|/Game/Blueprints/Tiles/Tile_Blank.Tile_Blank_C|SetisTilePlaced _selectedtile false))))

(event Custom|EventBind
  (bind _editorhud (Variables|Default|GetEditorHud))
  (EventDispatchers|BindEventtoSpawnActor _editorhud (delegate Custom|CreateTile))
  (EventDispatchers|BindEventtoDeleteTileButton _editorhud (delegate Custom|DeleteTile)))

(event Custom|CreateTile
  (params (Class :type Actor%20Class%20Reference))
  (bind _selectedtile (Variables|Default|GetSelectedTile))
  (if (Variables|Default|GetHoldingTile)
    (if (not (Variables|/Game/Blueprints/Tiles/Tile_Blank.Tile_Blank_C|GetisTilePlaced _selectedtile))
      (bind _returnvalue (Game|SpawnActorfromClass Class (Transformation|GetWorldTransform (Variables|/Game/Blueprints/Tiles/Tile_Blank.Tile_Blank_C|GetSceneRoot _selectedtile)) "Undefined" 0 0))
      (Variables|/Game/Blueprints/Tiles/Tile_Blank.Tile_Blank_C|SetisTilePlaced _selectedtile true)
      (Variables|/Game/Blueprints/Tiles/Tile_Blank.Tile_Blank_C|SetPlacedTile _selectedtile _returnvalue))))

(event EventBeginPlay
  (Utilities|FlowControl|Sequence
    (:then_0
      (for _index (range 0 20)
        (for _index_2 (range 0 20)
          (Game|SpawnActorfromClass "/Game/Blueprints/Tiles/Tile_Blank.Tile_Blank_C" (Math|Transform|MakeTransform (Math|Vector|MakeVector 0.0 (* _index 2e+02) (* _index_2 2e+02))) "Undefined" self 0))))
    (:then_1
      (bind _returnvalue (UserInterface|CreateWidget "/Game/Blueprints/UI/BP_UI_LevelEditor.BP_UI_LevelEditor_C"))
      (bind _output_get (Variables|Default|SetEditorHud _returnvalue))
      (UserInterface|Viewport|AddtoViewport _output_get 0))
    (:then_2
      (CallFunction|EventBind))
    (:then_3
      (Input|SetInputModeGameOnly (Game|GetPlayerController 0)))
    (:then_4
      (bind _returnvalue_2 (Actor|GetActorOfClass "/Game/Blueprints/LevelManager.LevelManager_C"))
      (Variables|Default|SetLevelManager _returnvalue_2))))

(event Input|AxisEvents|InputAxisRight
  (params (AxisValue :type Float%20%28single-precision%29))
  (Class|SceneComponent|AddWorldTransform (Variables|Collision|GetCapsuleComponent) (Math|Transform|MakeTransform (Math|Vector|MakeVector 0.0 (* (Variables|Default|GetMovementSpeed) AxisValue) 0.0) "0, 0, 0" "1,1,1") false false))

(event Input|AxisEvents|InputAxisUp
  (params (AxisValue :type Float%20%28single-precision%29))
  (Class|SceneComponent|AddWorldTransform (Variables|Collision|GetCapsuleComponent) (Math|Transform|MakeTransform (Math|Vector|MakeVector 0.0 0.0 (* (Variables|Default|GetMovementSpeed) AxisValue)) "0, 0, 0" "1,1,1") false false))

(event Input|AxisEvents|InputAxisNumKey
  (params (AxisValue :type Float%20%28single-precision%29))
  (bind _returnvalue (Math|Float|Truncate AxisValue))
  (bind _editorhud (Variables|Default|GetEditorHud))
  (bind _returnvalue_2 (- _returnvalue 1))
  (bind _buttonarr (Variables|/Game/Blueprints/UI/BP_UI_LevelEditor.BP_UI_LevelEditor_C|GetButtonArr _editorhud))
  (bind _output (Utilities|Array|Get(acopy) _buttonarr _returnvalue_2))
  (if (> _returnvalue 0)
    (Default|CallButtonWasClicked _output _returnvalue_2 (Variables|/Game/Blueprints/UI/BP_UI_EditorSlot.BP_UI_EditorSlot_C|GetItem _output))))

(event Input|MouseEvents|MouseWheelAxis
  (params (AxisValue :type Float%20%28single-precision%29))
  (Class|SceneComponent|AddWorldTransform (Variables|Collision|GetCapsuleComponent) (Math|Transform|MakeTransform (Math|Vector|MakeVector (* (* (Variables|Default|GetMovementSpeed) 2.0) AxisValue) 0.0 0.0) "0, 0, 0" "1,1,1") false false))

(event Input|KeyboardEvents|CtrlS
  (params (Key :type Key%20Structure :default "None"))
  (bind _editorhud (Variables|Default|GetEditorHud))
  (bind _levelmanager (Variables|Default|GetLevelManager))
  (:Pressed
    (Variables|/Game/Blueprints/LevelManager.LevelManager_C|SetLevelName _levelmanager (Utilities|String|ToString(Text) (Variables|/Game/Blueprints/UI/BP_UI_LevelEditor.BP_UI_LevelEditor_C|GetLevelNameText _editorhud)))
    (Variables|/Game/Blueprints/LevelManager.LevelManager_C|SetLevelCreator _levelmanager (Utilities|String|ToString(Text) (Variables|/Game/Blueprints/UI/BP_UI_LevelEditor.BP_UI_LevelEditor_C|GetLevelCreatorText _editorhud)))
    (Default|SaveLevel (Variables|Default|GetLevelManager))))

(event Input|KeyboardEvents|CtrlR
  (params (Key :type Key%20Structure :default "None"))
  (bind _editorhud (Variables|Default|GetEditorHud))
  (bind _levelmanager (Variables|Default|GetLevelManager))
  (:Pressed
    (Default|Loadlev (Variables|Default|GetLevelManager))
    (Variables|/Game/Blueprints/UI/BP_UI_LevelEditor.BP_UI_LevelEditor_C|SetLevelNameText _editorhud (Utilities|Text|ToText(String) (Variables|/Game/Blueprints/LevelManager.LevelManager_C|GetLevelName _levelmanager)))
    (Variables|/Game/Blueprints/UI/BP_UI_LevelEditor.BP_UI_LevelEditor_C|SetLevelCreatorText _editorhud (Utilities|Text|ToText(String) (Variables|/Game/Blueprints/LevelManager.LevelManager_C|GetLevelCreator _levelmanager)))))

(event Input|KeyboardEvents|CtrlQ
  (params (Key :type Key%20Structure :default "None"))
  (:Pressed
    (Default|NextLev (Variables|Default|GetLevelManager))))

(event Input|KeyboardEvents|0
  (params (Key :type Key%20Structure :default "None"))
  (:Pressed
    (CallFunction|DeleteTile)))

(fn ConstructionScript)