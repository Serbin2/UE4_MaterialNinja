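; Player character for a material-based ninja game, moving along one axis, jumping even mid-air, and throwing shurikens.
; A data-table row, initially Wood, sets movement physics and mesh material, which each shuriken inherits.
; BeginPlay moves the player to PlayerStartPoint, stores the respawn transform in the game mode, adds the HUD and counts stars.
; Tick respawns on falls or star completion, while hotkeys save and load levels through LevelManager.
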(event OnComponentHit(CapsuleComponent)
  (params (HitComponent :type Primitive%20Component%20Object%20Reference) (OtherActor :type Actor%20Object%20Reference) (OtherComp :type Primitive%20Component%20Object%20Reference) (NormalImpulse :type Vector :default "0, 0, 0") (Hit :type Hit%20Result%20Structure%20%28by%20ref%29))
  (if (AI|Components|NavMovement|IsMovingonGround (Variables|Character|GetCharacterMovement))
    (Development|PrintString "moving")))

(event Custom|LevelStart
  (bind _outactors (Actor|GetAllActorsOfClass "/Game/Blueprints/Items/BP_PickStar.BP_PickStar_C"))
  (Variables|Default|SetTotalStar (Utilities|Array|Length _outactors)))

(event EventBeginPlay
  (bind _capsulecomponent (Variables|Collision|GetCapsuleComponent))
  (Utilities|FlowControl|Sequence
    (:then_0
      (bind _returnvalue (Actor|GetActorOfClass "/Game/Blueprints/PlayerStartPoint.PlayerStartPoint_C"))
      (Utilities|IsValid _returnvalue
        (:Is%20Valid
          (Transformation|SetWorldTransform _capsulecomponent (Transformation|GetWorldTransform (Variables|/Game/Blueprints/PlayerStartPoint.PlayerStartPoint_C|GetSceneRoot _returnvalue)) false true)
          (Transformation|AddWorldOffset _capsulecomponent "0, 0,100.000000" false true)
          (Actor|DestroyActor _returnvalue))))
    (:then_1
      (Variables|Default|SetCurMatName "Wood")
      (CallFunction|GetMaterialInfo))
    (:then_2
      (bind _returnvalue_2 (UserInterface|CreateWidget "/Game/Blueprints/UI/BP_UI_HUD.BP_UI_HUD_C"))
      (bind _output_get (Variables|Default|SetHUDref _returnvalue_2))
      (UserInterface|Viewport|AddtoViewport _output_get 0))
    (:then_3
      (bind _asmaterial_ninja_gamemode (Utilities|Casting|CastToMaterialNinjaGamemode (Game|GetGameMode)))
      (bind _output_get_2 (Variables|Default|SetGameMode _asmaterial_ninja_gamemode))
      (Variables|/Game/Blueprints/MaterialNinjaGamemode.MaterialNinjaGamemode_C|SetPlayerStartPoint _output_get_2 (Transformation|GetActorTransform)))
    (:then_4
      (Input|SetInputModeGameOnly (Game|GetPlayerController 0)))
    (:then_5
      (CallFunction|LevelStart))))

(event EventTick
  (params (DeltaSeconds :type Float%20%28single-precision%29))
  (Utilities|FlowControl|Sequence
    (:then_0
      ;[1 1 1] player fall check and respawn
      (if (< (.z (Transformation|GetActorLocation)) -1e+02)
        (Development|PrintString "Dead")
        (CallFunction|RespawnSelf)))
    (:then_1
      (if (== (Variables|Default|GetTotalStar) (Variables|Default|GetCollectedStar))
        (Variables|Default|SetCollectedStar 0)
        (Pawn|Components|CharacterMovement|DisableMovement (Variables|Character|GetCharacterMovement))
        (Development|PrintString "Clear!")
        (Utilities|FlowControl|Delay 5.0)
        (CallFunction|RespawnSelf)
        (Pawn|Components|CharacterMovement|SetMovementMode (Variables|Character|GetCharacterMovement) "MOVE_Walking" 0)))))

(event Input|ActionEvents|InputActionJump
  (params (Key :type Key%20Structure :default "None"))
  ;[1 1 1] player controll
  (:Pressed
    (if (AI|Components|NavMovement|IsFalling (Variables|Character|GetCharacterMovement))
      (Pawn|Components|CharacterMovement|SetMovementMode (Variables|Character|GetCharacterMovement) "MOVE_Walking" 0)
      (Character|Jump)
      (else
        (Character|Jump))))
  (:Released
    (Character|StopJumping)))

(event Input|AxisEvents|InputAxisRight
  (params (AxisValue :type Float%20%28single-precision%29))
  ;[1 1 1] player controll
  (Pawn|Input|AddMovementInput "0,1.000000, 0" AxisValue false)
  (Variables|Default|SetAxis%20Value AxisValue)
  (Variables|Default|SetMovementSize (* "0,1.000000, 0" AxisValue)))

(event Input|KeyboardEvents|CtrlS
  (params (Key :type Key%20Structure :default "None"))
  ;[1 1 1] player controll
  (:Pressed
    (bind _returnvalue (Actor|GetActorOfClass "/Game/Blueprints/LevelManager.LevelManager_C"))
    (Default|SaveLevel _returnvalue)))

(event Input|KeyboardEvents|G
  (params (Key :type Key%20Structure :default "None"))
  (bind _myinfo (Variables|Default|GetMyInfo))
  (:Pressed
    (bind _returnvalue (Game|SpawnActorfromClass "/Game/Blueprints/Shuriken.Shuriken_C" (Transformation|GetWorldTransform (Variables|Collision|GetCapsuleComponent)) "Undefined" 0 0))
    (Variables|/Game/Blueprints/Shuriken.Shuriken_C|SetMyMatInfo _returnvalue _myinfo)
    (Rendering|Material|SetMaterial (Variables|/Game/Blueprints/Shuriken.Shuriken_C|GetMesh _returnvalue) 0 (.Material (Utilities|Struct|BreakMaterialInfo _myinfo)))))

(event Input|KeyboardEvents|CtrlR
  (params (Key :type Key%20Structure :default "None"))
  ;[1 1 1] player controll
  (:Pressed
    (bind _returnvalue (Actor|GetActorOfClass "/Game/Blueprints/LevelManager.LevelManager_C"))
    (Default|Loadlev _returnvalue)))

(fn ConstructionScript)

(fn RespawnSelf
  (Transformation|SetWorldTransform (Variables|Collision|GetCapsuleComponent) (Variables|/Game/Blueprints/MaterialNinjaGamemode.MaterialNinjaGamemode_C|GetPlayerStartPoint (Variables|Default|GetGameMode)) false true)
  (Variables|Default|SetCollectedStar 0)
  (Default|RespawnPlayer (Variables|Default|GetGameMode)))

(fn GetMaterialInfo
  (bind _charactermovement (Variables|Character|GetCharacterMovement))
  (bind _returnvalue (Utilities|GetDataTableRow "/Game/Blueprints/MaterialInfoTable.MaterialInfoTable" (Variables|Default|GetCurMatName))
    (:then
      (Utilities|FlowControl|Sequence
        (:then_0
          (Variables|/Script/Engine.CharacterMovementComponent|SetGravityScale _charactermovement (.GravityScale (Utilities|Struct|BreakMaterialInfo _returnvalue))))
        (:then_1
          (Variables|/Script/Engine.CharacterMovementComponent|SetMaxWalkSpeed _charactermovement (.WalkSpeed (Utilities|Struct|BreakMaterialInfo _returnvalue))))
        (:then_2
          (Variables|/Script/Engine.CharacterMovementComponent|SetJumpZVelocity _charactermovement (.JumpSpeed (Utilities|Struct|BreakMaterialInfo _returnvalue))))
        (:then_3
          (Variables|/Script/Engine.CharacterMovementComponent|SetAirControl _charactermovement (.AirControl (Utilities|Struct|BreakMaterialInfo _returnvalue))))
        (:then_4
          (Rendering|Material|SetMaterial (Variables|Character|GetMesh) 0 (.Material (Utilities|Struct|BreakMaterialInfo _returnvalue))))
        (:then_5
          (Variables|Default|SetMyInfo _returnvalue))))))