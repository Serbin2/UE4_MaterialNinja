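; ClassTable is a Blueprint that holds a material texture table and a level table, and handles level progression and retries.
; FindTextureSetByName searches the texture table by material name and falls back to the first entry when nothing matches.
; ClearCurrentLevel increments the current index and opens that level, or TestMainLevel once the index is out of range.
; RetryCurrentLevel reopens the level at the current index.
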(fn FindTextureSetbyName
  (params (Name :type Name))
  (bind _materialtexturetable (Variables|Default|GetMaterialTextureTable))
  (for _array_element _materialtexturetable
    (if (Utilities|Name|Equal(Name) Name (.MatName (Utilities|Struct|BreakMaterialTexSet _array_element)))
      (return _array_element)))
  (return (Utilities|Array|Get(acopy) _materialtexturetable)))

(fn ClearCurrentLevel
  (bind _leveltable (Variables|Default|GetLevelTable))
  (bind _output_get (Variables|Default|SetCurLevelIndex (+ (Variables|Default|GetCurLevelIndex) 1)))
  (if (Utilities|Array|IsValidIndex _leveltable _output_get)
    (Game|OpenLevel(byObjectReference) (Utilities|Array|Get(acopy) _leveltable _output_get))
    (else
      (Game|OpenLevel(byName) "TestMainLevel"))))

(fn RetryCurrentLevel
  (Game|OpenLevel(byObjectReference) (Utilities|Array|Get(acopy) (Variables|Default|GetLevelTable) (Variables|Default|GetCurLevelIndex))))