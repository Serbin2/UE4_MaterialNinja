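; Player character for the Material Ninja game, whose graph holds only its startup setup.
; On BeginPlay it moves to the PlayerStartPoint actor's mesh transform, destroys that actor, and records its own transform in MaterialNinjaGamemode as the start point.
; It also creates a dynamic material instance on the character mesh, adds the HUD, sets game-only input and stores an actor count as TotalStar.
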(event EventBeginPlay
  (bind _character_mesh (Variables|Default|GetCharacter%20Mesh))
  (Utilities|FlowControl|Sequence
    (:then_0
      ;[1 1 1] Character Transform Initialize
      (bind _returnvalue (Actor|GetActorOfClass "/Game/Blueprints/PlayerStartPoint.PlayerStartPoint_C"))
      (Utilities|IsValid _returnvalue
        (:Is%20Valid
          (Transformation|SetWorldTransform (Variables|Default|GetDefaultSceneRoot) (Transformation|GetWorldTransform (Variables|/Game/Blueprints/PlayerStartPoint.PlayerStartPoint_C|GetStaticMesh _returnvalue)) false true)
          (Actor|DestroyActor _returnvalue))))
    (:then_1
      ;[1 1 1] Get Dynamic Material Instance
      (bind _returnvalue_2 (Rendering|Material|CreateDynamicMaterialInstance _character_mesh 0 (Rendering|Material|GetMaterial _character_mesh 0) "None" :!class /Script/Engine.PrimitiveComponent))
      (Variables|Default|SetMatInst _returnvalue_2))
    (:then_2
      ;[1 1 1] HUD Set
      (bind _returnvalue_3 (UserInterface|CreateWidget "/Game/Blueprints/UI/BP_UI_HUD.BP_UI_HUD_C"))
      (bind _output_get (Variables|Default|SetHUD _returnvalue_3))
      (UserInterface|Viewport|AddtoViewport _output_get 0))
    (:then_3
      ;[1 1 1] Game Initialize
      (bind _asmaterial_ninja_gamemode (Utilities|Casting|CastToMaterialNinjaGamemode (Game|GetGameMode)))
      (bind _output_get_2 (Variables|Default|SetGameMode _asmaterial_ninja_gamemode))
      (Variables|/Game/Blueprints/MaterialNinjaGamemode.MaterialNinjaGamemode_C|SetPlayerStartPoint _output_get_2 (Transformation|GetActorTransform))
      (Input|SetInputModeGameOnly (Game|GetPlayerController 0)))
    (:then_4
      (bind _outactors (Actor|GetAllActorsOfClass 0))
      (Variables|Default|SetTotalStar (Utilities|Array|Length _outactors)))))

(fn ConstructionScript)