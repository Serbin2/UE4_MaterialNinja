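; Floor tile that breaks when a sufficiently heavy player stands directly on top of it.
; While the player overlaps it, a looping timer repeatedly runs CalculateAngle, which measures the angle between the player-to-tile direction and world up.
; If the player is almost straight above and their material's MassLevel is high enough, the tile destroys itself.
; Otherwise it nudges its TileBox with sine and cosine offsets to shake it.
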(event EventBeginPlay)

(event Collision|EventActorBeginOverlap
  (params (OtherActor :type Actor%20Object%20Reference))
  (bind _asplayer_character (Utilities|Casting|CastToPlayerCharacter OtherActor))
  (Variables|Default|SetPlayer _asplayer_character)
  (Utilities|Time|SetTimerbyFunctionName 0 "CalculateAngle" (/ 1.0 16.0) true))

(event EventTick
  (params (DeltaSeconds :type Float%20%28single-precision%29)))

(event Collision|EventActorEndOverlap
  (params (OtherActor :type Actor%20Object%20Reference))
  (if (== OtherActor (Variables|Default|GetPlayer))
    (Utilities|Time|ClearTimerbyFunctionName 0 "CalculateAngle")))

(fn ConstructionScript)

(fn CalculateAngle
  (bind _returnvalue (Actor|GetGameTimeSinceCreation))
  (bind _player (Variables|Default|GetPlayer))
  (if (> (Class|KismetMathLibrary|DegAcos (Math|Vector|DotProduct (Math|Vector|Normalize (- (Transformation|GetWorldLocation (Variables|Default|GetTileBox)) (Transformation|GetWorldLocation (Variables|/Script/Engine.Character|GetCapsuleComponent _player)))) (Math|Vector|GetUpVector "0, 0, 0"))) 1.7e+02)
    (if (> (.massLevel (Utilities|Struct|BreakNinjaMaterial (Variables|/Script/Nitest.BaseMatCharacter|GetMyMaterial _player))) 1)
      (Actor|DestroyActor)
      (else
        (Transformation|AddWorldOffset (Variables|Default|GetTileBox) (Math|Vector|MakeVector 0.0 (* (Math|Trig|Sin(Radians) (* _returnvalue 2e+01)) 2.5) (* (Math|Trig|Cos(Radians) (* _returnvalue 1e+01)) 1.5)) false false :!label _label)))
    (else
      (goto _label))))