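; Selectable tile for the level editor that highlights on cursor hover and click through the Alpha parameter of a dynamic material.
; Clicking toggles selection and updates the held tile state on the LevelEditorCharacter, first unselecting any tile it already holds.
; Unselect reuses the click toggle logic.
; A collision component's begin and end overlaps set and clear IsTilePlaced.
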(event OnBeginCursorOver(TileCube)
  (params (TouchedComponent :type Primitive%20Component%20Object%20Reference))
  (if (not (Variables|Default|GetisSelected))
    (Rendering|Material|SetScalarParameterValue (Variables|Default|GetMatInst) "Alpha" 0.2 :!class /Script/Engine.MaterialInstanceDynamic)))

(event OnComponentBeginOverlap(PlacedCheckCollision)
  (params (OverlappedComponent :type Primitive%20Component%20Object%20Reference) (OtherActor :type Actor%20Object%20Reference) (OtherComp :type Primitive%20Component%20Object%20Reference) (OtherBodyIndex :type Integer) (bFromSweep :type Boolean) (SweepResult :type Hit%20Result%20Structure%20%28by%20ref%29))
  (Variables|Default|SetisTilePlaced true))

(event OnClicked(TileCube)
  (params (TouchedComponent :type Primitive%20Component%20Object%20Reference) (ButtonPressed :type Key%20Structure :default "None"))
  (bind _player (Variables|Default|GetPlayer))
  (bind _matinst (Variables|Default|GetMatInst))
  (if (Variables|Default|GetisSelected)
    (Rendering|Material|SetScalarParameterValue _matinst "Alpha" 0.0 :!class /Script/Engine.MaterialInstanceDynamic)
    (Variables|Default|SetisSelected false)
    (Variables|/Game/Blueprints/LevelEditorCharacter.LevelEditorCharacter_C|SetHoldingTile (Variables|Default|GetPlayer) false)
    (else
      (if (Variables|/Game/Blueprints/LevelEditorCharacter.LevelEditorCharacter_C|GetHoldingTile (Variables|Default|GetPlayer))
        (CallFunction|Unselect (Variables|/Game/Blueprints/LevelEditorCharacter.LevelEditorCharacter_C|GetSelectedTile (Variables|Default|GetPlayer))))
      (Rendering|Material|SetScalarParameterValue _matinst "Alpha" 1.0 :!class /Script/Engine.MaterialInstanceDynamic)
      (bind _output_get (Variables|Default|SetisSelected true))
      (Variables|/Game/Blueprints/LevelEditorCharacter.LevelEditorCharacter_C|SetSelectedTile _player self)
      (Variables|/Game/Blueprints/LevelEditorCharacter.LevelEditorCharacter_C|SetHoldingTile _player _output_get))))

(event OnEndCursorOver(TileCube)
  (params (TouchedComponent :type Primitive%20Component%20Object%20Reference))
  (if (not (Variables|Default|GetisSelected))
    (Rendering|Material|SetScalarParameterValue (Variables|Default|GetMatInst) "Alpha" 0.0 :!class /Script/Engine.MaterialInstanceDynamic)))

(event OnComponentEndOverlap(PlacedCheckCollision)
  (params (OverlappedComponent :type Primitive%20Component%20Object%20Reference) (OtherActor :type Actor%20Object%20Reference) (OtherComp :type Primitive%20Component%20Object%20Reference) (OtherBodyIndex :type Integer))
  (Variables|Default|SetisTilePlaced false))

(event Custom|Unselect
  (bind _player (Variables|Default|GetPlayer))
  (bind _matinst (Variables|Default|GetMatInst))
  (if (Variables|Default|GetisSelected)
    (Rendering|Material|SetScalarParameterValue _matinst "Alpha" 0.0 :!class /Script/Engine.MaterialInstanceDynamic)
    (Variables|Default|SetisSelected false)
    (Variables|/Game/Blueprints/LevelEditorCharacter.LevelEditorCharacter_C|SetHoldingTile (Variables|Default|GetPlayer) false)
    (else
      (if (Variables|/Game/Blueprints/LevelEditorCharacter.LevelEditorCharacter_C|GetHoldingTile (Variables|Default|GetPlayer))
        (CallFunction|Unselect (Variables|/Game/Blueprints/LevelEditorCharacter.LevelEditorCharacter_C|GetSelectedTile (Variables|Default|GetPlayer))))
      (Rendering|Material|SetScalarParameterValue _matinst "Alpha" 1.0 :!class /Script/Engine.MaterialInstanceDynamic)
      (bind _output_get (Variables|Default|SetisSelected true))
      (Variables|/Game/Blueprints/LevelEditorCharacter.LevelEditorCharacter_C|SetSelectedTile _player self)
      (Variables|/Game/Blueprints/LevelEditorCharacter.LevelEditorCharacter_C|SetHoldingTile _player _output_get))))

(event EventBeginPlay
  (bind _returnvalue (Rendering|Material|CreateDynamicMaterialInstance (Variables|Default|GetTileCube) 0 "/Game/Materials/M_TP.M_TP" "None" :!class /Script/Engine.PrimitiveComponent))
  (Variables|Default|SetMatInst _returnvalue)
  (bind _returnvalue_2 (Actor|GetActorOfClass "/Game/Blueprints/LevelEditorCharacter.LevelEditorCharacter_C"))
  (Variables|Default|SetPlayer _returnvalue_2))

(fn ConstructionScript)