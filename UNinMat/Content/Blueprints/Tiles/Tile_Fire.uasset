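; Fire hazard tile that affects players and material boxes vulnerable to fire when they overlap its box collider.
; A player flagged WeakFire respawns, while a WeakFire MaterialBox is disabled and added to the MaterialNinjaGamemode's DisabledActor list.
; The construction script gives the mesh a dynamic M_Fire material instance.
; Timelines meant to drive its UTile and VTile parameters are unconnected and never run.
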(event OnComponentBeginOverlap(BoxCollider)
  (params (OverlappedComponent :type Primitive%20Component%20Object%20Reference) (OtherActor :type Actor%20Object%20Reference) (OtherComp :type Primitive%20Component%20Object%20Reference) (OtherBodyIndex :type Integer) (bFromSweep :type Boolean) (SweepResult :type Hit%20Result%20Structure%20%28by%20ref%29))
  (bind _asplayer_character (Utilities|Casting|CastToPlayerCharacter OtherActor)
    (:then
      (if (.weakfire (Variables|/Game/Blueprints/PlayerCharacter.PlayerCharacter_C|GetMyInfo _asplayer_character))
        (Development|PrintString "Dead")
        (Default|RespawnSelf _asplayer_character)))
    (:CastFailed
      (bind _asmaterial_box (Utilities|Casting|CastToMaterialBox OtherActor))
      (if (.weakfire (Variables|/Game/Blueprints/MaterialBox.MaterialBox_C|GetMyMatInfo _asmaterial_box))
        (CallFunction|DisableActor _asmaterial_box)
        (bind _asmaterial_ninja_gamemode (Utilities|Casting|CastToMaterialNinjaGamemode (Game|GetGameMode)))
        (Utilities|Array|Add (Variables|/Game/Blueprints/MaterialNinjaGamemode.MaterialNinjaGamemode_C|GetDisabledActor _asmaterial_ninja_gamemode) _asmaterial_box)
        (Development|PrintString "BoxDisabled")))))

(event EventBeginPlay)

(event EventTick
  (params (DeltaSeconds :type Float%20%28single-precision%29)))

(fn ConstructionScript
  (bind _returnvalue (Rendering|Material|CreateDynamicMaterialInstance (Variables|Default|GetStaticMesh) 0 "/Game/Materials/M_Fire.M_Fire" "" :!class /Script/Engine.PrimitiveComponent))
  (Variables|Default|SetMatVal _returnvalue))