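; Fire tile hazard that respawns the player character when it overlaps the tile.
; Overlap casts to the player, prints a debug message and sets a named timer for MaterialCollide, which calls RespawnSelf.
; The construction script gives the cube a dynamic fire material; timelines meant to drive its U and V tiling are never triggered.
; BeginPlay caches the ninja game mode, which is otherwise unused here.
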(event EventBeginPlay
  (bind _asninja_gamemode (Utilities|Casting|CastToNinjaGamemode (Game|GetGameMode)))
  (Variables|Default|SetAs%20Ninja%20Gamemode _asninja_gamemode))

(event Collision|EventActorBeginOverlap
  (params (OtherActor :type Actor%20Object%20Reference))
  (bind _asbase_mat_character (Utilities|Casting|CastToBaseMatCharacter OtherActor))
  (bind _asplayer_character (Utilities|Casting|CastToPlayerCharacter _asbase_mat_character))
  (Development|PrintString "Hello")
  (Utilities|Time|SetTimerbyFunctionName 0 "MaterialCollide" 0.0))

(event EventTick
  (params (DeltaSeconds :type Float%20%28single-precision%29)))

(event EventMaterialCollide
  (params (target :type Actor%20Object%20Reference))
  (Default|RespawnSelf (stale Collision|EventActorBeginOverlap _asplayer_character)))

(fn ConstructionScript
  (bind _returnvalue (Rendering|Material|CreateDynamicMaterialInstance (Variables|Default|GetTileCube) 0 "/Game/Materials/M_Fire.M_Fire" "" :!class /Script/Engine.PrimitiveComponent))
  (Variables|Default|SetMatVal _returnvalue))