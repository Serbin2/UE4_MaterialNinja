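; MaterialEffect provides a MaterialChange function that matches a mesh's look and mass level to the material type held by a NinjaMaterial.
; It switches on the MyMaterial value (None, Paper, Wood, Stone or Iron), sets the mesh's first material slot and writes MassLevel back to NinjaMaterial.
; Mass level rises from None through Stone, Iron shares Stone's level, and None uses an ocean water material.
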(fn MaterialChange
  (params (Mesh :type Primitive%20Component%20Object%20Reference) (NinjaMaterial :type Ninja%20Material%20Component%20Object%20Reference))
  (switch Utilities|FlowControl|Switch|SwitchonENinijaMaterial (Variables|/Script/Nitest.NinjaMaterialComponent|GetmyMaterial NinjaMaterial)
    (:eNone
      (Rendering|Material|SetMaterial Mesh 0 "/Game/StarterContent/Materials/M_Water_Ocean.M_Water_Ocean")
      (Variables|/Script/Nitest.NinjaMaterialComponent|SetmassLevel NinjaMaterial 0))
    (:ePaper
      (Rendering|Material|SetMaterial Mesh 0 "/Game/Materials/M_Paper.M_Paper")
      (Variables|/Script/Nitest.NinjaMaterialComponent|SetmassLevel NinjaMaterial 1))
    (:eWood
      (Rendering|Material|SetMaterial Mesh 0 "/Game/Materials/M_Wood.M_Wood")
      (Variables|/Script/Nitest.NinjaMaterialComponent|SetmassLevel NinjaMaterial 2))
    (:eStone
      (Rendering|Material|SetMaterial Mesh 0 "/Game/Materials/M_Rock.M_Rock")
      (Variables|/Script/Nitest.NinjaMaterialComponent|SetmassLevel NinjaMaterial 3 :!label _label))
    (:eIron
      (Rendering|Material|SetMaterial Mesh 0 "/Game/Materials/M_Iron.M_Iron")
      (goto _label))))