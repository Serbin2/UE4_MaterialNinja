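; Game mode for a ninja game that respawns the player and resets the collectible stars.
; A one-time pass on Tick caches the transforms of all placed BP_PickStar meshes in StarArr.
; RespawnPlayer spawns and possesses a new character at the start point, replaces all stars from that cache and resets the character's star counts.
; The MaterialFactory setup is unconnected and never runs.
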(event Custom|RespawnPlayer
  (bind _returnvalue (Game|SpawnActorfromClass "/Game/Blueprints/PlayerCharacter.PlayerCharacter_C" (Variables|Default|GetPlayerStartPoint) "Undefined" 0 0))
  (Pawn|Possess (Game|GetPlayerController 0) _returnvalue)
  (bind _outactors (Actor|GetAllActorsOfClass "/Game/Blueprints/Items/BP_PickStar.BP_PickStar_C"))
  (for _array_element _outactors
    (Actor|DestroyActor _array_element))
  (CallFunction|RespawnStar)
  (Variables|/Game/Blueprints/PlayerCharacter.PlayerCharacter_C|SetCollectedStar _returnvalue 0)
  (Variables|/Game/Blueprints/PlayerCharacter.PlayerCharacter_C|SetTotalStar _returnvalue (Utilities|Array|Length (Variables|Default|GetStarArr))))

(event Custom|RespawnStar
  (for _array_element (Variables|Default|GetStarArr)
    (Game|SpawnActorfromClass "/Game/Blueprints/Items/BP_PickStar.BP_PickStar_C" _array_element "Undefined" 0 0)))

(event EventBeginPlay)

(event EventTick
  (params (DeltaSeconds :type Float%20%28single-precision%29))
  (Utilities|FlowControl|DoOnce false
    (:Completed
      (bind _outactors (Actor|GetAllActorsOfClass "/Game/Blueprints/Items/BP_PickStar.BP_PickStar_C"))
      (for _array_element _outactors
        (Utilities|Array|Add (Variables|Default|GetStarArr) (Transformation|GetWorldTransform (Variables|/Game/Blueprints/Items/BP_PickStar.BP_PickStar_C|GetMesh _array_element)))))))

(fn ConstructionScript)