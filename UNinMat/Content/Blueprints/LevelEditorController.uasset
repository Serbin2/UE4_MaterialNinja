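; LevelEditorController handles input for what its name indicates is a level editor, covering pausing and mouse clicks.
; The Pause action lazily creates and caches a BP_UI_PopupMenu widget, adds it to the viewport, shows the cursor, switches to UI-only input and pauses the game.
; Left click only prints debug text: "clicked" and the name of the actor under the cursor, found by a complex Visibility trace.
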(event EventBeginPlay)

(event EventTick
  (params (DeltaSeconds :type Float%20%28single-precision%29)))

(event Input|ActionEvents|InputActionPause
  (params (Key :type Key%20Structure :default "None"))
  (bind _returnvalue (Game|GetPlayerController 0))
  (:Pressed
    (Utilities|IsValid (Variables|Default|GetPopupMenuRef)
      (:Is%20Valid
        _)
      (:Is%20Not%20Valid
        (bind _returnvalue_2 (UserInterface|CreateWidget "/Game/Blueprints/UI/BP_UI_PopupMenu.BP_UI_PopupMenu_C"))
        (Variables|Default|SetPopupMenuRef _returnvalue_2)))
    (Variables|/Script/Engine.PlayerController|SetbShowMouseCursor _returnvalue true)
    (Input|SetInputModeUIOnly _returnvalue (Variables|Default|GetPopupMenuRef) "DoNotLock")
    (UserInterface|Viewport|AddtoViewport (Variables|Default|GetPopupMenuRef) 0)
    (Game|SetGamePaused true)))

(event Input|MouseEvents|LeftMouseButton
  (params (Key :type Key%20Structure :default "None"))
  (:Pressed
    (Development|PrintString "clicked")
    (Development|PrintString (Utilities|GetDisplayName (.hitactor (.HitResult (Game|Player|GetHitResultUnderCursorbyChannel "TraceTypeQuery1" true)))))))

(fn ConstructionScript)