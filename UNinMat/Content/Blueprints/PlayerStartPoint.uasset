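; PlayerStartPoint is a placeable actor that marks where the player starts in a level.
; On BeginPlay under MaterialNinjaGamemode, it writes its transform into the game mode's PlayerStartPoint variable.
; Under LevelEditorGamemode, it instead destroys every other PlayerStartPoint actor, so a newly spawned one replaces any existing start point.
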(event EventBeginPlay
  (bind _returnvalue (Game|GetGameMode))
  (bind _asmaterial_ninja_gamemode (Utilities|Casting|CastToMaterialNinjaGamemode _returnvalue)
    (:then
      (Variables|/Game/Blueprints/MaterialNinjaGamemode.MaterialNinjaGamemode_C|SetPlayerStartPoint _asmaterial_ninja_gamemode (Transformation|GetActorTransform)))
    (:CastFailed
      (Utilities|Casting|CastToLevelEditorGamemode _returnvalue)
      (bind _outactors (Actor|GetAllActorsOfClass "PlayerStartPoint_C"))
      (for _array_element _outactors
        (if (not (== _array_element self))
          (Actor|DestroyActor _array_element))))))

(fn ConstructionScript)