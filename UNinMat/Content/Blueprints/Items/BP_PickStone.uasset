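; Stone material pickup that switches the player character's ninja material to Stone on touch.
; Its mesh spins in yaw by a fixed step each tick, independent of frame time.
; When a PlayerCharacter overlaps the Box, it changes that character's NinjaMaterial to EStone, calls MaterialChange on the character mesh and sets the material name.
; The pickup is not destroyed or disabled afterwards.
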(event OnComponentBeginOverlap(Box)
  (params (OverlappedComponent :type Primitive%20Component%20Object%20Reference) (OtherActor :type Actor%20Object%20Reference) (OtherComp :type Primitive%20Component%20Object%20Reference) (OtherBodyIndex :type Integer) (bFromSweep :type Boolean) (SweepResult :type Hit%20Result%20Structure%20%28by%20ref%29))
  (bind _asplayer_character (Utilities|Casting|CastToPlayerCharacter OtherActor))
  (Class|NinjaMaterialComponent|ChangeMaterial (Variables|/Script/Nitest.BaseMatCharacter|GetNinjaMaterial _asplayer_character) "eStone")
  (CallFunction|MaterialChange (Variables|/Script/Engine.Character|GetMesh _asplayer_character) (Variables|/Script/Nitest.BaseMatCharacter|GetNinjaMaterial _asplayer_character))
  (Variables|/Script/Nitest.NinjaMaterialComponent|SetMaterialName (Variables|/Script/Nitest.BaseMatCharacter|GetNinjaMaterial _asplayer_character) "Stone"))

(event EventBeginPlay)

(event Collision|EventActorBeginOverlap
  (params (OtherActor :type Actor%20Object%20Reference)))

(event EventTick
  (params (DeltaSeconds :type Float%20%28single-precision%29))
  (bind _mesh (Variables|Default|GetMesh))
  (bind _relativerotation (Variables|/Script/Engine.SceneComponent|GetRelativeRotation _mesh))
  (bind (_roll _pitch _yaw) (Math|Rotator|BreakRotator _relativerotation))
  (Transformation|SetRelativeRotation _mesh (Math|Rotator|MakeRotator _roll _pitch (+ _yaw 1.0)) false false))

(fn ConstructionScript)