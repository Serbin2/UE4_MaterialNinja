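; Water trigger actor that turns an overlapping PlayerCharacter into the Water material and switches its capsule collision channel.
; It drives the material by rebinding the player's MaterialTick event, acting as a small state machine.
; WaterTick switches to Steam when the player touches fire.
; SteamTick pushes the player upward in Falling mode up to a speed cap, while a DoOnce-gated delay reverts it to Water after three seconds.
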(event OnComponentBeginOverlap(Box)
  (params (OverlappedComponent :type Primitive%20Component%20Object%20Reference) (OtherActor :type Actor%20Object%20Reference) (OtherComp :type Primitive%20Component%20Object%20Reference) (OtherBodyIndex :type Integer) (bFromSweep :type Boolean) (SweepResult :type Hit%20Result%20Structure%20%28by%20ref%29))
  (bind _asplayer_character (Utilities|Casting|CastToPlayerCharacter OtherActor))
  (if (Utilities|Name|NotEqual(Name) (Variables|/Game/Blueprints/PlayerCharacter.PlayerCharacter_C|GetCurMatName _asplayer_character) "Water")
    (Variables|/Game/Blueprints/PlayerCharacter.PlayerCharacter_C|SetCurMatName _asplayer_character "Water")
    (Collision|SetCollisionObjectType (Variables|/Script/Engine.Character|GetCapsuleComponent _asplayer_character) "ECC_GameTraceChannel2")
    (Default|GetMaterialInfo _asplayer_character)
    (EventDispatchers|UnbindallEventsfromMaterialTick _asplayer_character)
    (EventDispatchers|BindEventtoMaterialTick _asplayer_character (delegate Custom|WaterTick))))

(event Custom|WaterTick
  (bind _issteam (CallFunction|WaterTickFunc))
  (if _issteam
    (EventDispatchers|BindEventtoMaterialTick (stale OnComponentBeginOverlap(Box) _asplayer_character) (delegate Custom|SteamTick))))

(event Custom|SteamTick
  (bind _as_player_character (Variables|Default|GetAs%20Player%20Character))
  (bind _as_player_character_2 (Variables|Default|GetAs%20Player%20Character))
  (bind _charactermovement (Variables|/Script/Engine.Character|GetCharacterMovement _as_player_character_2))
  (Utilities|FlowControl|Sequence
    (:then_0
      (Utilities|FlowControl|DoOnce false :!label _label
        (:Completed
          (Utilities|FlowControl|Delay 3.0)
          (Variables|/Game/Blueprints/PlayerCharacter.PlayerCharacter_C|SetCurMatName _as_player_character "Water")
          (Default|GetMaterialInfo _as_player_character)
          (EventDispatchers|UnbindallEventsfromMaterialTick _as_player_character)
          (Utilities|FlowControl|Sequence
            (:then_0
              (goto _label Reset))
            (:then_1
              (EventDispatchers|BindEventtoMaterialTick (stale OnComponentBeginOverlap(Box) _asplayer_character) (delegate Custom|WaterTick)))))))
    (:then_1
      (Pawn|Components|CharacterMovement|SetMovementMode _charactermovement "MOVE_Falling" 0)
      (if (< (.Z (Math|Vector|BreakVector (Variables|/Script/Engine.MovementComponent|GetVelocity _charactermovement))) 8e+02)
        (Variables|/Script/Engine.MovementComponent|SetVelocity _charactermovement (+ (Variables|/Script/Engine.MovementComponent|GetVelocity _charactermovement) "0, 0,100.000000"))))))

(event EventBeginPlay)

(event Collision|EventActorBeginOverlap
  (params (OtherActor :type Actor%20Object%20Reference)))

(event EventTick
  (params (DeltaSeconds :type Float%20%28single-precision%29)))

(fn ConstructionScript)

(fn WaterTickFunc
  (Utilities|FlowControl|Sequence
    (:then_0
      (Utilities|FlowControl|DoOnce false
        (:Completed
          (bind _asplayer_character (Utilities|Casting|CastToPlayerCharacter (Game|Player|GetPlayerPawn 0)))
          (Variables|Default|SetAs%20Player%20Character _asplayer_character))))
    (:then_1
      (if (Variables|/Game/Blueprints/PlayerCharacter.PlayerCharacter_C|GetisFireTouched (Variables|Default|GetAs%20Player%20Character))
        (Variables|/Game/Blueprints/PlayerCharacter.PlayerCharacter_C|SetCurMatName (Variables|Default|GetAs%20Player%20Character) "Steam")
        (Default|GetMaterialInfo (Variables|Default|GetAs%20Player%20Character))
        (EventDispatchers|UnbindallEventsfromMaterialTick (Variables|Default|GetAs%20Player%20Character))
        (return true)
        (else
          (return false))))))