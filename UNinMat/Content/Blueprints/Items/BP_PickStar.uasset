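; BP_PickStar is a collectible star pickup that increases the player's star count when touched.
; Tick spins the mesh by a fixed yaw step each frame, so its speed depends on frame rate.
; When a PlayerCharacter overlaps the Box, the star increments that character's CollectedStar, prints the new total and destroys itself.
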(event OnComponentBeginOverlap(Box)
  (params (OverlappedComponent :type Primitive%20Component%20Object%20Reference) (OtherActor :type Actor%20Object%20Reference) (OtherComp :type Primitive%20Component%20Object%20Reference) (OtherBodyIndex :type Integer) (bFromSweep :type Boolean) (SweepResult :type Hit%20Result%20Structure%20%28by%20ref%29))
  (bind _asplayer_character (Utilities|Casting|CastToPlayerCharacter OtherActor))
  (bind _output_get (Variables|/Game/Blueprints/PlayerCharacter.PlayerCharacter_C|SetCollectedStar _asplayer_character (+ (Variables|/Game/Blueprints/PlayerCharacter.PlayerCharacter_C|GetCollectedStar _asplayer_character) 1)))
  (Development|PrintString (Utilities|String|ToString(Integer) _output_get))
  (Actor|DestroyActor))

(event EventBeginPlay)

(event Collision|EventActorBeginOverlap
  (params (OtherActor :type Actor%20Object%20Reference)))

(event EventTick
  (params (DeltaSeconds :type Float%20%28single-precision%29))
  (bind _mesh (Variables|Default|GetMesh))
  (bind _returnvalue (Transformation|GetWorldRotation _mesh))
  (bind (_roll _pitch _yaw) (Math|Rotator|BreakRotator _returnvalue))
  (Transformation|SetWorldRotation _mesh (Math|Rotator|MakeRotator _roll _pitch (+ _yaw 1.0)) false false))

(fn ConstructionScript)