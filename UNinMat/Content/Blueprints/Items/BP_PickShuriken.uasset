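; BP_PickShuriken is a pickup item that gives the player one extra shuriken.
; Tick spins the static mesh around yaw by a fixed step per frame, independent of delta time.
; When a PlayerCharacter overlaps the Box, it increments RemainShuriken and disables itself rather than being destroyed.
; It then registers itself in the MaterialNinjaGamemode's DisabledActor list.
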(event OnComponentBeginOverlap(Box)
  (params (OverlappedComponent :type Primitive%20Component%20Object%20Reference) (OtherActor :type Actor%20Object%20Reference) (OtherComp :type Primitive%20Component%20Object%20Reference) (OtherBodyIndex :type Integer) (bFromSweep :type Boolean) (SweepResult :type Hit%20Result%20Structure%20%28by%20ref%29))
  (bind _self self)
  (bind _asplayer_character (Utilities|Casting|CastToPlayerCharacter OtherActor))
  (Variables|/Game/Blueprints/PlayerCharacter.PlayerCharacter_C|SetRemainShuriken _asplayer_character (+ (Variables|/Game/Blueprints/PlayerCharacter.PlayerCharacter_C|GetRemainShuriken _asplayer_character) 1))
  (CallFunction|DisableActor _self)
  (bind _asmaterial_ninja_gamemode (Utilities|Casting|CastToMaterialNinjaGamemode (Game|GetGameMode)))
  (Utilities|Array|Add (Variables|/Game/Blueprints/MaterialNinjaGamemode.MaterialNinjaGamemode_C|GetDisabledActor _asmaterial_ninja_gamemode) _self))

(event EventBeginPlay)

(event Collision|EventActorBeginOverlap
  (params (OtherActor :type Actor%20Object%20Reference)))

(event EventTick
  (params (DeltaSeconds :type Float%20%28single-precision%29))
  (bind _staticmesh (Variables|Default|GetStaticMesh))
  (bind _relativerotation (Variables|/Script/Engine.SceneComponent|GetRelativeRotation _staticmesh))
  (bind (_roll _pitch _yaw) (Math|Rotator|BreakRotator _relativerotation))
  (Transformation|SetRelativeRotation _staticmesh (Math|Rotator|MakeRotator _roll _pitch (+ _yaw 1.0)) false false))

(fn ConstructionScript)